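; Door actor for a button puzzle that moves up to open and down to close.
; On BeginPlay it looks up a BP_Button in the level and binds its Open and Close events to that button's dispatchers.
; Each event plays a 2D sound and uses MoveComponentTo to shift the static mesh vertically by a fixed offset, feeding world transforms into the relative targets.
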(event Custom|Open
  (bind _staticmeshcomponent (Variables|Debug|GetStaticMeshComponent))
  (Audio|PlaySound2D "/Engine/VREditor/Sounds/UI/Click_on_Button.Click_on_Button" 1.0 1.0 0.0 0 0)
  (Components|MoveComponentTo _staticmeshcomponent (+ (Transformation|GetWorldLocation _staticmeshcomponent) "0.000000,0.000000,500.000000") (Transformation|GetWorldRotation (Variables|Debug|GetStaticMeshComponent)) false false 0.2 false))

(event Custom|Close
  (bind _staticmeshcomponent (Variables|Debug|GetStaticMeshComponent))
  (Audio|PlaySound2D "/Engine/VREditor/Sounds/UI/Floating_UI_Close-001.Floating_UI_Close-001" 1.0 1.0 0.0 0 0)
  (Components|MoveComponentTo _staticmeshcomponent (- (Transformation|GetWorldLocation _staticmeshcomponent) "0.000000,0.000000,500.000000") (Transformation|GetWorldRotation (Variables|Debug|GetStaticMeshComponent)) false false 0.0 false))

(event EventBeginPlay
  (Actor|GetActorOfClass "/Game/Blueprint/PuzzleDoorFix/BP_Button.BP_Button_C")
  (bind _output_get (Variables|Default|SetButtonRef (Variables|Default|GetButton%20Ref)))
  (EventDispatchers|BindEventtoOpen _output_get (delegate Custom|Open))
  (EventDispatchers|BindEventtoClose _output_get (delegate Custom|Close)))

(fn ConstructionScript)