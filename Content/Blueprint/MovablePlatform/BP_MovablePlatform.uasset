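; BP_MovablePlatform is a platform that can be set to move between two editable locations.
; The Construction Script, when CanMove is enabled, fills the InterpToMovement component's control points with Location1 and Location2, both relative to the actor.
; It also applies the Duration variable to that component, so the path and timing are configured per instance without any event logic.
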(fn ConstructionScript
  (bind _interptomovement (Variables|Default|GetInterpToMovement))
  ;[1 1 1] Movimento editabile del bersaglio
  (if (Variables|Default|GetCanMove)
    (Variables|/Script/Engine.InterpToMovementComponent|SetControlPoints _interptomovement (Utilities|Array|MakeArray (Utilities|Struct|MakeInterpControlPoint (Variables|Default|GetLocation1) true) (Utilities|Struct|MakeInterpControlPoint (Variables|Default|GetLocation2) true)))
    (Variables|/Script/Engine.InterpToMovementComponent|SetDuration _interptomovement (Variables|Default|GetDuration))))