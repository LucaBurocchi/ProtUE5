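; Puzzle door actor that raises and lowers its static mesh in response to a BP_Button.
; On BeginPlay it looks up a BP_Button in the level and binds Open and Close to that button's events.
; Each event uses MoveComponentTo to shift the mesh vertically by a fixed offset from its current position, passing world location and rotation as the relative targets.
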(event Custom|Open
  (bind _staticmeshcomponent (Variables|Debug|GetStaticMeshComponent))
  (Components|MoveComponentTo _staticmeshcomponent (+ (Transformation|GetWorldLocation _staticmeshcomponent) "0.000000,0.000000,500.000000") (Transformation|GetWorldRotation (Variables|Debug|GetStaticMeshComponent)) false false 0.2 false))

(event Custom|Close
  (bind _staticmeshcomponent (Variables|Debug|GetStaticMeshComponent))
  (Components|MoveComponentTo _staticmeshcomponent (- (Transformation|GetWorldLocation _staticmeshcomponent) "0.000000,0.000000,500.000000") (Transformation|GetWorldRotation (Variables|Debug|GetStaticMeshComponent)) false false 0.0 false))

(event EventBeginPlay
  (Actor|GetActorOfClass "/Game/Blueprint/PuzzleDoor/BP_Button.BP_Button_C")
  (bind _output_get (Variables|Default|SetButtonRef (Variables|Default|GetButton%20Ref)))
  (EventDispatchers|BindEventtoOpen _output_get (delegate Custom|Open))
  (EventDispatchers|BindEventtoClose _output_get (delegate Custom|Close)))

(fn ConstructionScript)