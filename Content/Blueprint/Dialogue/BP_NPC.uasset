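; BP_NPC is a talkable NPC that shows its dialogue lines one at a time in an on-screen widget.
; The construction script fills the name text from CharacterName, and SetInteractableState shows or hides it.
; Each Talk call advances TalkIndex through Dialogue, reusing a lazily created WB_Dialogue and calling a 2D sound, then removes the widget after the last line.
; TalkIndex is never reset here, and EventTalk2 is empty.
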(event Custom|EventTalk2)

(event EventSetInteractableState
  (params (bCanShowInteract? :type Boolean))
  ;[1 1 1] Comparsa/ scomparsa nome NPC
  (if bCanShowInteract?
    (Rendering|SetVisibility (Variables|Default|GetTxt_CharacterName) true false)
    (else
      (Rendering|SetVisibility (Variables|Default|GetTxt_CharacterName) false false))))

(event EventTalk
  (Math|Integer|IncrementInt (Variables|Default|GetTalkIndex)
    (:%20%20
      (if (< (Variables|Default|GetTalkIndex) (Utilities|Array|Length (Variables|Default|GetDialogue)))
        (Variables|Default|GetUI
          (:then
            _)
          (:else
            (bind _returnvalue (UserInterface|CreateWidget "/Game/Blueprint/Dialogue/WB_Dialogue.WB_Dialogue_C" (Game|GetPlayerController 0)))
            (bind _output_get (Variables|Default|SetUI _returnvalue))))
        (UserInterface|Viewport|AddtoViewport _output_get 0)
        (Rendering|Components|TextRender|SetText (Variables|/Game/Blueprint/Dialogue/WB_Dialogue.WB_Dialogue_C|GetTalkText (Variables|Default|GetUI)) (Utilities|Text|ToText(String) (Utilities|Array|Get(acopy) (Variables|Default|GetDialogue) (Variables|Default|GetTalkIndex))))
        ;[1 1 1] inserire suono
        (Audio|PlaySound2D 0 1.0 1.0 0.0 0 0)
        (else
          (Widget|RemovefromParent (Variables|Default|GetUI)))))))

(fn ConstructionScript
  (Rendering|Components|TextRender|SetText (Variables|Default|GetTxt_CharacterName) (Variables|Default|GetCharacterName)))